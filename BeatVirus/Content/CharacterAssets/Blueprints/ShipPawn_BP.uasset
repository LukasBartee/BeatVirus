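; Player ship pawn whose body mesh is moved by dragging a finger or the mouse.
; Touch or left-click stores a screen anchor plus the previous offset, and touch moves or the FingerMovement axis update the offset from it, printing it for debugging.
; Tick sets the mesh's relative location to actor location plus that Y-flipped, unscaled pixel offset.
; An interpolated, swept world-space move is left unconnected.
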(event `self.ReceiveTick`
  (params (DeltaSeconds :type "Float (single-precision)"))
  (bind (_currentoffset_x _currentoffset_y _currentoffset_z) (`KismetMathLibrary.BreakVector` (`self.CurrentOffset`)))
  (`SceneComponent.K2_SetRelativeLocation` (`self.PlayerBodyMesh`) (+ (`self.K2_GetActorLocation`) (`KismetMathLibrary.MakeVector` _currentoffset_x (* _currentoffset_y -1.0) _currentoffset_z)) false false))

(event `InputTouch`
  (params (Location :type "Vector Structure") (FingerIndex :type "ETouchIndex Enum"))
  (bind (_currentscreenlocation_x _currentscreenlocation_y _currentscreenlocation_z) (`KismetMathLibrary.BreakVector` (`self.CurrentScreenLocation`)))
  (bind (_locationx _locationy) (`PlayerController.GetInputTouchState` (`GameplayStatics.GetPlayerController` 0) "Touch1"))
  (:`Pressed`
    (bind _output_get (set `self.CurrentScreenLocation` (`KismetMathLibrary.MakeVector` 0.0 _locationx _locationy)))
    (set `self.CurrentScreenLocation` (+ _output_get (`self.CurrentOffset`))))
  (:`Moved`
    (bind _output_get_2 (set `self.CurrentOffset` (`KismetMathLibrary.MakeVector` 0.0 (- _currentscreenlocation_y _locationx) (- _currentscreenlocation_z _locationy))))
    (`KismetSystemLibrary.PrintString` (`KismetStringLibrary.Conv_VectorToString` _output_get_2))))

(event `Key|LeftMouseButton`
  (params (Key :type "Key Structure"))
  (bind _returnvalue (`GameplayStatics.GetPlayerController` 0))
  (bind (_locationx _locationy) (`PlayerController.GetMousePosition` _returnvalue))
  (:`Pressed`
    (set `PlayerController.bShowMouseCursor` true _returnvalue)
    (bind _output_get (set `self.CurrentScreenLocation` (`KismetMathLibrary.MakeVector` 0.0 _locationx _locationy)))
    (set `self.CurrentScreenLocation` (+ _output_get (`self.CurrentOffset`)))))

(event `InputAxis|FingerMovement`
  (params (AxisValue :type "Float (single-precision)"))
  (bind (_currentscreenlocation_x _currentscreenlocation_y _currentscreenlocation_z) (`KismetMathLibrary.BreakVector` (`self.CurrentScreenLocation`)))
  (bind (_locationx _locationy) (`PlayerController.GetMousePosition` (`GameplayStatics.GetPlayerController` 0)))
  (if (> AxisValue 0.0)
    (bind _output_get (set `self.CurrentOffset` (`KismetMathLibrary.MakeVector` 0.0 (- _currentscreenlocation_y _locationx) (- _currentscreenlocation_z _locationy))))
    (`KismetSystemLibrary.PrintString` (`KismetStringLibrary.Conv_VectorToString` _output_get))))

(fn `UserConstructionScript`)