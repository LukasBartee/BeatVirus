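; Unfinished procedural tube actor prototype that currently only visualizes computed vertex positions with a debug sphere.
; On BeginPlay it loops over Subdivisions with a Delay, accumulating a Z-rotated radius vector into VertexCarrier via RotateAround.
; Each step offsets the sphere by that accumulated vector and prints a message.
; The CurrentRotation increment and ProcTube mesh-section creation are unconnected, so the angle stays fixed and no mesh is built.
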(event Collision|EventActorBeginOverlap
  (params (OtherActor :type Actor%20Object%20Reference)))

(event EventTick
  (params (DeltaSeconds :type Float%20%28single-precision%29)))

(event EventBeginPlay
  (bind _debugsphere (Variables|Default|GetDebugSphere))
  (for _index (range 0 (- (Variables|Default|GetSubdivisions) 1))
    (Utilities|FlowControl|Delay 1.0)
    (bind _newposition (CallFunction|RotateAround (Variables|Default|GetVertexCarrier) (Variables|Default|GetRadius) (stale _output_get)))
    (bind _output_get (Variables|Default|SetVertexCarrier _newposition))
    (Transformation|SetActorLocation _debugsphere (+ (Transformation|GetActorLocation _debugsphere) _output_get) false false)
    (Development|PrintString "Locationset")))

(fn ConstructionScript)

(fn RotateAround
  (params (Target%20Vector :type Vector) (Radius :type Float%20%28single-precision%29) (Angle :type Float%20%28single-precision%29))
  (LocalVariables|SetLVector Target%20Vector)
  (LocalVariables|SetLRadius Radius)
  (LocalVariables|SetLAngle Angle)
  (return (+ (LocalVariables|GetLVector) (Math|Vector|RotateVectorAroundAxis (Math|Vector|MakeVector (LocalVariables|GetLRadius) 0.0 0.0) (LocalVariables|GetLAngle) "0, 0,1.000000"))))